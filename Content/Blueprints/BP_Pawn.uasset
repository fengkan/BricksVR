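; BP_Pawn is a motion-controller pawn that spawns BP_Ball actors at either hand.
; Each controller trigger spawns a ball at its controller's location and stores it in one shared Ball variable.
; Both paths join a single two-second Delay, then enable physics on the stored ball's sphere and zero its velocity.
; Presses during the delay overwrite Ball, so only the latest ball gets released.
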(event `Key|MotionController_Left_Trigger`
  (params (Key :type "Key Structure" :default "AnyKey"))
  (bind _ball (`self.ball`))
  (:`Pressed`
    (bind _returnvalue (`|SpawnActorFromClass` "/Game/Blueprints/BP_Ball.BP_Ball_C" (`KismetMathLibrary.MakeTransform` (`SceneComponent.K2_GetComponentLocation` (`self.MotionController`))) "Undefined" "OverrideRootScale"))
    (set `self.ball` _returnvalue)
    (`KismetSystemLibrary.Delay` 2.0 :!label _label)
    (`PrimitiveComponent.SetSimulatePhysics` (`/Game/Blueprints/BP_Ball.Sphere` _ball) true)
    (`PrimitiveComponent.SetAllPhysicsLinearVelocity` (`/Game/Blueprints/BP_Ball.Sphere` _ball) (0.0 0.0 0.0) false)))

(event `Key|MotionController_Right_Trigger`
  (params (Key :type "Key Structure" :default "AnyKey"))
  (:`Pressed`
    (bind _returnvalue (`|SpawnActorFromClass` "/Game/Blueprints/BP_Ball.BP_Ball_C" (`KismetMathLibrary.MakeTransform` (`SceneComponent.K2_GetComponentLocation` (`self.MotionController1`))) "Undefined" "OverrideRootScale"))
    (set `self.ball` _returnvalue)
    (goto _label)))

(fn `UserConstructionScript`)